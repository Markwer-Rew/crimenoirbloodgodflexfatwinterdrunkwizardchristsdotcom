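; BP_RClue is a trigger volume that shows and hides the RClue hint on the player HUD.
; On BeginPlay it finds and caches the BP_PlayerHud actor in the level.
; When the first-person character enters the box it plays the RClue widget's Splash animation forward, and on exit it plays it in reverse.
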(event OnComponentBeginOverlap(Box)
  (params (OverlappedComponent :type Primitive%20Component%20Object%20Reference) (OtherActor :type Actor%20Object%20Reference) (OtherComp :type Primitive%20Component%20Object%20Reference) (OtherBodyIndex :type Integer) (bFromSweep :type Boolean) (SweepResult :type Hit%20Result%20Structure%20%28by%20ref%29))
  (bind _hud (Variables|Default|GetHud))
  (bind _rclue (Variables|/Game/UI/BP_PlayerHud.BP_PlayerHud_C|GetRClue _hud))
  (Utilities|Casting|CastToBP_FirstPersonCharacter OtherActor)
  (UserInterface|Animation|PlayAnimation _rclue (Variables|/Game/UI/WBP_RButtonClue.WBP_RButtonClue_C|GetSplash _rclue) 0.0 1 "Forward" 1.0 false))

(event OnComponentEndOverlap(Box)
  (params (OverlappedComponent :type Primitive%20Component%20Object%20Reference) (OtherActor :type Actor%20Object%20Reference) (OtherComp :type Primitive%20Component%20Object%20Reference) (OtherBodyIndex :type Integer))
  (bind _hud (Variables|Default|GetHud))
  (bind _rclue (Variables|/Game/UI/BP_PlayerHud.BP_PlayerHud_C|GetRClue _hud))
  (Utilities|Casting|CastToBP_FirstPersonCharacter OtherActor)
  (UserInterface|Animation|PlayAnimation _rclue (Variables|/Game/UI/WBP_RButtonClue.WBP_RButtonClue_C|GetSplash _rclue) 0.0 1 "Reverse" 1.0 false))

(event EventBeginPlay
  (bind _returnvalue (Actor|GetActorOfClass "/Game/UI/BP_PlayerHud.BP_PlayerHud_C"))
  (Variables|Default|SetHud _returnvalue))

(fn ConstructionScript)