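; BP_HungryButton is a trigger button with a door that must be fed objects before it opens and leads to another level.
; While hungry, it destroys overlapping WinCondition-tagged actors until their count reaches Colvo.
; Once fed, a further tagged overlap plays a timeline rotating the door open, and any end overlap reverses it.
; A second box loads the target level when BP_FirstPersonCharacter enters while the door is flagged open.
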(event OnComponentBeginOverlap(Box)
  (params (OverlappedComponent :type Primitive%20Component%20Object%20Reference) (OtherActor :type Actor%20Object%20Reference) (OtherComp :type Primitive%20Component%20Object%20Reference) (OtherBodyIndex :type Integer) (bFromSweep :type Boolean) (SweepResult :type Hit%20Result%20Structure%20%28by%20ref%29))
  (if (Actor|ActorHasTag OtherActor "WinCondition")
    (if (Variables|Default|GetisDoorHungry)
      (Actor|DestroyActor OtherActor)
      (Variables|Default|SetHanger (+ (Variables|Default|GetHanger) 1.0))
      (if (>= (Variables|Default|GetHanger) (Variables|Default|GetCol-vo))
        (Variables|Default|SetisDoorHungry false))
      (else
        (Variables|Default|SetDoorOpend true)
        (bind _newtrack_0 (Timeline|Door PlayFromStart)
          (:Update
            (Transformation|SetRelativeRotation (Variables|Default|GetScene) (Math|Rotator|MakeRotator 0.0 0.0 _newtrack_0) false false)))))))

(event OnComponentEndOverlap(Box)
  (params (OverlappedComponent :type Primitive%20Component%20Object%20Reference) (OtherActor :type Actor%20Object%20Reference) (OtherComp :type Primitive%20Component%20Object%20Reference) (OtherBodyIndex :type Integer))
  (Variables|Default|SetDoorOpend false)
  (bind _newtrack_0 (Timeline|Door Reverse)
    (:Update
      (Transformation|SetRelativeRotation (Variables|Default|GetScene) (Math|Rotator|MakeRotator 0.0 0.0 _newtrack_0) false false))))

(event OnComponentBeginOverlap(Box1)
  (params (OverlappedComponent :type Primitive%20Component%20Object%20Reference) (OtherActor :type Actor%20Object%20Reference) (OtherComp :type Primitive%20Component%20Object%20Reference) (OtherBodyIndex :type Integer) (bFromSweep :type Boolean) (SweepResult :type Hit%20Result%20Structure%20%28by%20ref%29))
  (Utilities|Casting|CastToBP_FirstPersonCharacter OtherActor)
  (if (Variables|Default|GetDoorOpend)
    (Game|OpenLevel(byObjectReference) (Variables|Default|GetLevel))))

(fn ConstructionScript)